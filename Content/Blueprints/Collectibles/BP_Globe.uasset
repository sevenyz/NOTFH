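; BP_Globe is a health pickup collectible that restores a percentage of the player character's maximum HP.
; Its sphere collider's begin overlap responds only to components tagged PlayerCollider on a FinalProjectAlphaCharacter, then adds the HpPercentageToAdd share of MaxHP to CurrentHP, capped at MaxHP.
; After healing, it plays a 2D collection sound and destroys itself.
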(event `self.SphereCollider.OnComponentBeginOverlap`
  (params (OverlappedComponent :type "PrimitiveComponent Object Reference") (OtherActor :type "Actor Object Reference") (OtherComp :type "PrimitiveComponent Object Reference") (OtherBodyIndex :type Integer) (bFromSweep :type Boolean) (SweepResult :type "HitResult Structure (by ref)"))
  (if (`ActorComponent.ComponentHasTag` OtherComp "PlayerCollider")
    (bind _asfinal_project_alpha_character (cast `FinalProjectAlphaCharacter` OtherActor))
    (bind _maxhp (`FinalProjectAlphaCharacter.MaxHP` _asfinal_project_alpha_character))
    (bind _returnvalue (+ (* (/ _maxhp 100.0) (`self.HpPercentageToAdd`)) (`FinalProjectAlphaCharacter.CurrentHP` _asfinal_project_alpha_character)))
    (set `FinalProjectAlphaCharacter.CurrentHP` (select `bool` (<= _returnvalue _maxhp) :`false` _maxhp :`true` _returnvalue) _asfinal_project_alpha_character)
    (`GameplayStatics.PlaySound2D` "/Game/Sounds/Player/Collection_HP_Sound_NOTFH.Collection_HP_Sound_NOTFH" 1.0 1.0 0.0 null null)
    (`self.K2_DestroyActor`)))

(fn `UserConstructionScript`)