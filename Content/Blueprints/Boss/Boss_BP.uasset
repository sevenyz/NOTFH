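; Wolf boss character whose events play attack, trap-stun and hit montages, and whose death pauses the game on a win screen.
; It reports player-behind, stun, hit and line-of-sight states to its AI blackboard, and has an AOE damage function.
; Incoming combo increments restart a timer that, on expiry, converts the count into bleeding, blind (zeroed attack damage) or timed poison.
; Each effect claims a free icon slot in the boss HP widget.
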(event `self.ReceiveBeginPlay`
  (bind (_direction _newtrack_0) (`Timeline|Timeline_0`)
    (:`Update`
      (`SceneComponent.K2_SetRelativeLocation` (`self.Cone`) (`KismetMathLibrary.MakeVector` 0.0 0.0 _newtrack_0) false false)
      (bind _foundwidgets (`WidgetBlueprintLibrary.GetAllWidgetsOfClass` "/Game/Hud/UI_BossHP.UI_BossHP_C" false))
      (set `self.UI_Boss` (`|GetArrayItem` _foundwidgets)))))

(event `self.ReceiveTick`
  (params (DeltaSeconds :type "Float (single-precision)")))

(event `EventAttack`
  ;[0 0 0] Attack
  (`|PlayMontage` (`self.Mesh`) (select `int` (`KismetMathLibrary.RandomIntegerInRange` 0 1) :`0` "/Game/Characters/Wolf/Animations/Attack_Left_Wolf_Montage.Attack_Left_Wolf_Montage" :`1` "/Game/Characters/Wolf/Animations/Attack_Right_Wolf_Montage.Attack_Right_Wolf_Montage" :!type "AnimMontage Object Reference") 1.5
    (:`OnCompleted`
      (`SkeletalMeshComponent.SetAnimationMode` (`self.Mesh`) "AnimationBlueprint")
      (`/Engine/EditorBlueprintResources/StandardMacros.IncrementInt` (`self.AttacksDoneCount`)))))

(event `self.BackCollider.OnComponentBeginOverlap`
  (params (OverlappedComponent :type "PrimitiveComponent Object Reference") (OtherActor :type "Actor Object Reference") (OtherComp :type "PrimitiveComponent Object Reference") (OtherBodyIndex :type Integer) (bFromSweep :type Boolean) (SweepResult :type "HitResult Structure (by ref)"))
  (if (`ActorComponent.ComponentHasTag` OtherComp "PlayerCollider")
    (`BlackboardComponent.SetValueAsBool` (`AIBlueprintHelperLibrary.GetBlackboard` (`self.GetController`)) "IsPlayerBehind" true)))

(event `AttackRotate`
  ;[0 0 0] Attack
  (`|PlayMontage` (`self.Mesh`) "/Game/Characters/Wolf/Animations/Wolf_attack_rotate_Montage.Wolf_attack_rotate_Montage" 1.5
    (:`OnCompleted`
      (`SkeletalMeshComponent.SetAnimationMode` (`self.Mesh`) "AnimationBlueprint"))))

(event `self.BackCollider.OnComponentEndOverlap`
  (params (OverlappedComponent :type "PrimitiveComponent Object Reference") (OtherActor :type "Actor Object Reference") (OtherComp :type "PrimitiveComponent Object Reference") (OtherBodyIndex :type Integer))
  (if (`ActorComponent.ComponentHasTag` OtherComp "PlayerCollider")
    (`BlackboardComponent.SetValueAsBool` (`AIBlueprintHelperLibrary.GetBlackboard` (`self.GetController`)) "IsPlayerBehind" false)))

(event `ImpactAttack`
  ;[0 0 0] Attack
  (`|PlayMontage` (`self.Mesh`) "/Game/Characters/Wolf/Animations/Attack_04_Montage.Attack_04_Montage" 1.5
    (:`then`
      (set `self.AttacksDoneCount` 0))
    (:`OnCompleted`
      (`SkeletalMeshComponent.SetAnimationMode` (`self.Mesh`) "AnimationBlueprint"))))

(event `JumpAttack`
  ;[0 0 0] Attack
  (`|PlayMontage` (`self.Mesh`) "/Game/Characters/Wolf/Animations/Attack_05_Montage.Attack_05_Montage" 1.5
    (:`OnCompleted`
      (`SkeletalMeshComponent.SetAnimationMode` (`self.Mesh`) "AnimationBlueprint"))))

(event `EventTrapped`
  (bind _returnvalue (`GameplayStatics.SpawnEmitterAtLocation` "/Game/Particles/Stun_Particle/Stun_Ps.Stun_Ps" (`SceneComponent.K2_GetComponentLocation` (`self.StunParticleLocation`))))
  (`|PlayMontage` (`self.Mesh`) "/Game/Characters/Wolf/Animations/TrapHitLoop_Wolf_Montage.TrapHitLoop_Wolf_Montage"
    (:`then`
      (`KismetSystemLibrary.Delay` (`self.StunTime`))
      (`ActorComponent.K2_DestroyComponent` _returnvalue)
      (if (not (`BlackboardComponent.GetValueAsBool` (`AIBlueprintHelperLibrary.GetBlackboard` (`self.GetController`)) "IsHit"))
        (`|PlayMontage` (`self.Mesh`) "/Game/Characters/Wolf/Animations/Attack_04_Montage.Attack_04_Montage"
          (:`OnCompleted`
            (set `self.bIsHit` false)
            (`BlackboardComponent.SetValueAsBool` (`AIBlueprintHelperLibrary.GetBlackboard` (`self.GetController`)) "IsStunned" false)
            (`BlackboardComponent.SetValueAsBool` (`AIBlueprintHelperLibrary.GetBlackboard` (`self.GetController`)) "IsHit" false)
            (`SkeletalMeshComponent.SetAnimationMode` (`self.Mesh`) "AnimationBlueprint")
            (`BlackboardComponent.SetValueAsBool` (`AIBlueprintHelperLibrary.GetBlackboard` (`self.GetController`)) "HasLineOfSight" true)))))))

(event `OnHit`
  (`SceneComponent.SetVisibility` (`self.HealthBarWidget`) true false)
  (`BlackboardComponent.SetValueAsBool` (`AIBlueprintHelperLibrary.GetBlackboard` (`self.GetController`)) "HasLineOfSight" true)
  (if (not (not (`self.bIsBombDamage`)))
    (if (not (`BlackboardComponent.GetValueAsBool` (`AIBlueprintHelperLibrary.GetBlackboard` (`self.GetController`)) "IsStunned"))
      (`|PlayMontage` (`self.Mesh`) "/Game/Characters/Wolf/Animations/TrapHitNoLoop_Wolf_Montage.TrapHitNoLoop_Wolf_Montage"
        (:`OnCompleted`
          _)))
    (`SkeletalMeshComponent.SetAnimationMode` (`self.Mesh`) "AnimationBlueprint")
    (set `self.bIsBombDamage` false)
    (`BlackboardComponent.SetValueAsBool` (`AIBlueprintHelperLibrary.GetBlackboard` (`self.GetController`)) "IsHit" false)
    (`BlackboardComponent.SetValueAsBool` (`AIBlueprintHelperLibrary.GetBlackboard` (`self.GetController`)) "HasLineOfSight" true)))

(event `ResetBleedingIcon`
  (bind _ui_boss (`self.UI_Boss`))
  (`KismetSystemLibrary.Delay` 2.0)
  (`WidgetSwitcher.SetActiveWidgetIndex` (select `int` (`self.BleedingIconIndex`) :`0` (`/Game/Hud/UI_BossHP.WS01` _ui_boss) :`1` (`/Game/Hud/UI_BossHP.WS02` _ui_boss) :`2` (`/Game/Hud/UI_BossHP.WS03` _ui_boss)) 0))

(event `self.Death`
  (bind _returnvalue (`GameplayStatics.GetPlayerController` 0))
  (`KismetSystemLibrary.PrintString` "Boss Is Dead")
  (bind _returnvalue_2 (`|CreateWidget` "/Game/Hud/WinScreen.WinScreen_C"))
  (`UserWidget.AddToViewport` _returnvalue_2 0)
  (`WidgetBlueprintLibrary.SetInputMode_UIOnlyEx` _returnvalue null)
  (set `PlayerController.bShowMouseCursor` true _returnvalue)
  (`GameplayStatics.SetGamePaused` true)
  (`self.K2_DestroyActor`))

(fn `ApplyStatusEffect`
  (switch `int` (`self.ComboCount`)
    (:`Default`
      (`self.Poison` :!label _label)
      (`KismetSystemLibrary.PrintString` "poison"))
    (:`1`
      _)
    (:`2`
      _)
    (:`3`
      (`self.Bleeding`)
      (`KismetSystemLibrary.PrintString` "bleeding"))
    (:`4`
      (`self.Blind`)
      (`KismetSystemLibrary.PrintString` "blind"))
    (:`5`
      (goto _label)))
  (set `self.ComboCount` 0)
  (`KismetSystemLibrary.PrintString` "end combo" true true (struct :`R` 1.0 :`B` 0.076571 :`A` 1.0)))

(fn `Bleeding`
  (locals (BleedingDamage :type "Float (double-precision)" :default 10.0))
  (set `self.CurrentHP` (- (`self.CurrentHP`) (/ (`self.MaxHP`) (`local.BleedingDamage`))))
  (bind _newparam (`self.SetStatusIcon` 1))
  (set `self.BleedingIconIndex` _newparam)
  (`self.ResetBleedingIcon`)
  (`GameplayStatics.SpawnEmitterAttached` "/Game/Particles/Blood/BloodSplat_PS.BloodSplat_PS" (`self.Mesh`) "pelvisSocket" (0.0 0.0 0.0) (struct) (1.5 1.5 1.5)))

(fn `Blind`
  (set `self.AttackDamage` 0)
  (bind _returnvalue (`KismetSystemLibrary.K2_SetTimer` self "StopBlind" 5.0))
  (set `self.BlindTimerHandle` _returnvalue)
  (`KismetSystemLibrary.PrintString` "blind on")
  (bind _newparam (`self.SetStatusIcon` 2))
  (set `self.BlindIconIndex` _newparam))

(fn `BossAOE`
  (bind (_returnvalue_x _returnvalue_y _returnvalue_z) (`KismetMathLibrary.BreakVector` (`self.K2_GetActorLocation`)))
  (`/Engine/EditorBlueprintResources/StandardMacros.IsValid` (`|GetArrayItem` (`PrimitiveComponent.GetOverlappingActors` (`self.AOE`) "/Game/Blueprints/Player/BP_Player.BP_Player_C"))
    (:`Is Valid`
      (`FinalProjectAlphaCharacter.TakeDamage` (`self.PlayerRef`) (`self.AttackDamage`)))
    (:`Is Not Valid`
      _))
  (`GameplayStatics.SpawnEmitterAtLocation` "/Game/Particles/Shockwave_AoE_BossAttack/AoE_Attack_PS.AoE_Attack_PS" (`KismetMathLibrary.MakeVector` _returnvalue_x _returnvalue_y (- _returnvalue_z 140.0))))

(fn `DecreaseHpOverTime`
  (bind _ui_boss (`self.UI_Boss`))
  (if (>= (`self.TimerCounter`) (`self.PoisonDuration`))
    (`KismetSystemLibrary.K2_ClearAndInvalidateTimerHandle` (`self.PoisonTimerHandle`))
    (`KismetSystemLibrary.PrintString` "stop poison")
    (`WidgetSwitcher.SetActiveWidgetIndex` (select `int` (`self.PoisonIconIndex`) :`0` (`/Game/Hud/UI_BossHP.WS01` _ui_boss) :`1` (`/Game/Hud/UI_BossHP.WS02` _ui_boss) :`2` (`/Game/Hud/UI_BossHP.WS03` _ui_boss)) 0)
    (else
      (bind _result (`/Engine/EditorBlueprintResources/StandardMacros.IncrementFloat` (`self.TimerCounter`))
        (:`  `
          (bind _output_get (set `self.CurrentHP` (- (`self.CurrentHP`) (`self.PoisonDamage`)))))))))

(fn `IncrementComboCount`
  (bind _result (`/Engine/EditorBlueprintResources/StandardMacros.IncrementInt` (`self.ComboCount`))
    (:`  `
      (`KismetSystemLibrary.PrintString` (`KismetStringLibrary.Conv_IntToString` _result))
      (`KismetSystemLibrary.K2_ClearAndInvalidateTimerHandle` (`self.TimerHandle`))
      (bind _returnvalue (`KismetSystemLibrary.K2_SetTimer` self "ApplyStatusEffect" 2.0))
      (set `self.TimerHandle` _returnvalue))))

(fn `Poison`
  (set `self.TimerCounter` 0.0)
  (`KismetSystemLibrary.K2_ClearAndInvalidateTimerHandle` (`self.PoisonTimerHandle`))
  (set `self.PoisonDamage` (* (`self.MaxHP`) (/ (`self.PoisonDamagePercentage`) 100.0)))
  (bind _returnvalue (`KismetSystemLibrary.K2_SetTimer` self "DecreaseHpOverTime" 1.0 true))
  (set `self.PoisonTimerHandle` _returnvalue)
  (bind _newparam (`self.SetStatusIcon` 3))
  (set `self.PoisonIconIndex` _newparam))

(fn `SetStatusIcon`
  (params (Index :type Integer))
  (returns (NewParam :type Integer))
  (locals (NewLocalVar_0 :type Integer))
  (bind _ui_boss (`self.UI_Boss`))
  (bind _ws02 (`/Game/Hud/UI_BossHP.WS02` _ui_boss))
  (bind _ws03 (`/Game/Hud/UI_BossHP.WS03` _ui_boss))
  (bind _ws01 (`/Game/Hud/UI_BossHP.WS01` _ui_boss))
  (if (== (`WidgetSwitcher.GetActiveWidgetIndex` _ws01) 0)
    (`WidgetSwitcher.SetActiveWidgetIndex` _ws01 Index)
    (set `local.NewLocalVar_0` 0)
    (return (`local.NewLocalVar_0`))
    (elif (== (`WidgetSwitcher.GetActiveWidgetIndex` _ws02) 0)
      (`WidgetSwitcher.SetActiveWidgetIndex` _ws02 Index)
      (set `local.NewLocalVar_0` 1)
      (return (`local.NewLocalVar_0`))
      (elif (== (`WidgetSwitcher.GetActiveWidgetIndex` _ws03) 0)
        (`WidgetSwitcher.SetActiveWidgetIndex` _ws03 Index)
        (set `local.NewLocalVar_0` 2)
        (return (`local.NewLocalVar_0`))))))

(fn `StopBlind`
  (bind _ui_boss (`self.UI_Boss`))
  (set `self.AttackDamage` (`self.MaxAttackDamage`))
  (`KismetSystemLibrary.K2_ClearAndInvalidateTimerHandle` (`self.BlindTimerHandle`))
  (`KismetSystemLibrary.PrintString` "stop blind")
  (`WidgetSwitcher.SetActiveWidgetIndex` (select `int` (`self.BlindIconIndex`) :`0` (`/Game/Hud/UI_BossHP.WS01` _ui_boss) :`1` (`/Game/Hud/UI_BossHP.WS02` _ui_boss) :`2` (`/Game/Hud/UI_BossHP.WS03` _ui_boss)) 0))

(fn `UpdateWalkSpeed`
  (params (NewWalkSpeed :type "Float (double-precision)"))
  (set `CharacterMovementComponent.MaxWalkSpeed` NewWalkSpeed (`self.CharacterMovement`)))

(fn `UserConstructionScript`)