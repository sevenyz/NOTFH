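; Thrown trap projectile that deploys the player's selected trap where it hits an actor tagged Landscape.
; On BeginPlay it caches BP_Player and copies its projectile movement initial speed to the player.
; On a landscape hit it reads the selected trap index at that moment, spawns a damage, stun or slow trap, then destroys itself.
; If collision prevents the spawn, that trap's counter on the player is incremented.
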(event `self.ReceiveBeginPlay`
  (bind _asbp_player (cast `/Game/Blueprints/Player/BP_Player` (`GameplayStatics.GetPlayerCharacter` 0)))
  (bind _output_get (set `self.PlayerRef` _asbp_player))
  (set `/Game/Blueprints/Player/BP_Player.ProjectileSpeed` (`ProjectileMovementComponent.InitialSpeed` (`self.ProjectileMovement`)) _output_get))

(event `self.Sphere1.OnComponentHit`
  (params (HitComponent :type "PrimitiveComponent Object Reference") (OtherActor :type "Actor Object Reference") (OtherComp :type "PrimitiveComponent Object Reference") (NormalImpulse :type "Vector Structure") (Hit :type "HitResult Structure (by ref)"))
  (bind _playerref (`self.PlayerRef`))
  (bind (_selectedtrap_traptype _selectedtrap_trapcost _selectedtrap_trapcounter _selectedtrap_trapindex) (break `TrapStats` (`FinalProjectAlphaCharacter.SelectedTrap` _playerref)))
  (bind (_output_traptype _output_trapcost _output_trapcounter) (break `TrapStats` (`|GetArrayItem` (`FinalProjectAlphaCharacter.TrapArray` (`self.PlayerRef`)) 2)))
  (bind (_output_traptype_2 _output_trapcost_2 _output_trapcounter_2) (break `TrapStats` (`|GetArrayItem` (`FinalProjectAlphaCharacter.TrapArray` (`self.PlayerRef`)))))
  (bind (_output_traptype_3 _output_trapcost_3 _output_trapcounter_3) (break `TrapStats` (`|GetArrayItem` (`FinalProjectAlphaCharacter.TrapArray` (`self.PlayerRef`)) 1)))
  (bind (_output_traptype_4 _output_trapcost_4 _output_trapcounter_4 _output_trapindex) (break `TrapStats` (`|GetArrayItem` (`FinalProjectAlphaCharacter.TrapArray` _playerref) _selectedtrap_trapindex)))
  (if (`self.ActorHasTag` OtherActor "Landscape")
    (set `self.SpawnPoint` (`KismetMathLibrary.Conv_VectorToTransform` Hit_ImpactPoint))
    (switch `int` _output_trapindex
      (:`0`
        (bind _output_get (set `self.TrapToSpawn` "/Game/Blueprints/Trap/DamageTrap_BP.DamageTrap_BP_C"))
        (bind _returnvalue (`|SpawnActorFromClass` _output_get (`self.SpawnPoint`) "AdjustIfPossibleButDontSpawnIfColliding" "OverrideRootScale" null null))
        (`/Engine/EditorBlueprintResources/StandardMacros.IsValid` _returnvalue
          (:`Is Valid`
            _)
          (:`Is Not Valid`
            (`/Engine/EditorBlueprintResources/StandardMacros.IncrementInt` _output_trapcounter_2
              (:`  `
                _))))
        (`self.K2_DestroyActor`))
      (:`1`
        (bind _output_get_2 (set `self.TrapToSpawn` "/Game/Blueprints/Trap/StunTrap_BP.StunTrap_BP_C"))
        (bind _returnvalue_2 (`|SpawnActorFromClass` _output_get_2 (`self.SpawnPoint`) "AdjustIfPossibleButDontSpawnIfColliding" "OverrideRootScale" null null))
        (`/Engine/EditorBlueprintResources/StandardMacros.IsValid` _returnvalue_2
          (:`Is Valid`
            _)
          (:`Is Not Valid`
            (`/Engine/EditorBlueprintResources/StandardMacros.IncrementInt` _output_trapcounter_3
              (:`  `
                _))))
        (`self.K2_DestroyActor`))
      (:`2`
        (bind _output_get_3 (set `self.TrapToSpawn` "/Game/Blueprints/Trap/SlowTrap_BP.SlowTrap_BP_C"))
        (bind _returnvalue_3 (`|SpawnActorFromClass` _output_get_3 (`self.SpawnPoint`) "AdjustIfPossibleButDontSpawnIfColliding" "OverrideRootScale" null null))
        (`/Engine/EditorBlueprintResources/StandardMacros.IsValid` _returnvalue_3
          (:`Is Valid`
            _)
          (:`Is Not Valid`
            (`/Engine/EditorBlueprintResources/StandardMacros.IncrementInt` _output_trapcounter
              (:`  `
                _))))
        (`self.K2_DestroyActor`)))))

(fn `UserConstructionScript`)