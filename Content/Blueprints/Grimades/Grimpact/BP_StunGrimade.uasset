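; BP_StunGrimade is a grenade that stuns the boss or minion its collider hits and can trigger Blood Drain.
; The first component tag selects the target, whose speed is zeroed for StunTime and rotation blocked.
; An already primed target turns on the player's Blood Drain for a delay while the collider is disabled and hidden; otherwise the hit primes it and resets its status.
; The grenade then destroys itself, as it does on a miss.
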(event `self.ReceiveBeginPlay`
  (`parent.ReceiveBeginPlay`))

(event `self.Collider.OnComponentHit`
  (params (HitComponent :type "PrimitiveComponent Object Reference") (OtherActor :type "Actor Object Reference") (OtherComp :type "PrimitiveComponent Object Reference") (NormalImpulse :type "Vector Structure") (Hit :type "HitResult Structure (by ref)"))
  (bind _stuntime (`self.StunTime`))
  (bind _playerref (`self.PlayerRef`))
  (bind _collider (`self.Collider`))
  (bind _bossref (`self.BossRef`))
  (bind _minionref (`self.MinionRef`))
  (bind _playerref_2 (`self.PlayerRef`))
  (bind _collider_2 (`self.Collider`))
  (switch `name` (`|GetArrayItem` (`ActorComponent.ComponentTags` OtherComp))
    (:`Default`
      (`KismetSystemLibrary.PrintString` "miss" :!label _label)
      (`self.K2_DestroyActor`))
    (:`BossCollider`
      (bind _asboss_bp (cast `/Game/Blueprints/Boss/Boss_BP` OtherActor))
      (bind _output_get (set `Boss.StunTime` _stuntime _asboss_bp))
      (`Boss.ChangeSpeed` _asboss_bp 0.0 _output_get)
      (`Boss.BlockRotation` _asboss_bp)
      (if (`/Game/Blueprints/Boss/Boss_BP.bCanApplyBloodDrain` _bossref)
        (`PrimitiveComponent.SetCollisionEnabled` _collider "NoCollision")
        (`SceneComponent.SetVisibility` _collider false true)
        (set `/Game/Blueprints/Player/BP_Player.bIsBloodDrainActive` true _playerref)
        (`KismetSystemLibrary.Delay` (`self.BloodDrainDuration`))
        (set `/Game/Blueprints/Player/BP_Player.bIsBloodDrainActive` false _playerref)
        (else
          (set `/Game/Blueprints/Boss/Boss_BP.bCanApplyBloodDrain` true _bossref)
          (`/Game/Blueprints/Boss/Boss_BP.ResetStatus` (`self.BossRef`))))
      (`self.K2_DestroyActor`))
    (:`MinionCollider`
      (bind _asnew_minion_bp (cast `/Game/Blueprints/Minion/NewMinion_BP` OtherActor))
      (bind _output_get_2 (set `self.MinionRef` _asnew_minion_bp))
      (bind _output_get_3 (set `NewMinion.StunTime` _stuntime _output_get_2))
      (`NewMinion.ChangeSpeed` _asnew_minion_bp 0.0 _output_get_3)
      (`NewMinion.BlockRotation` _asnew_minion_bp)
      (if (`/Game/Blueprints/Minion/NewMinion_BP.bCanApplyBloodDrain` _minionref)
        (`PrimitiveComponent.SetCollisionEnabled` _collider_2 "NoCollision")
        (`SceneComponent.SetVisibility` _collider_2 false true)
        (set `/Game/Blueprints/Player/BP_Player.bIsBloodDrainActive` true _playerref_2)
        (`KismetSystemLibrary.Delay` (`self.BloodDrainDuration`))
        (set `/Game/Blueprints/Player/BP_Player.bIsBloodDrainActive` false _playerref_2)
        (else
          (set `/Game/Blueprints/Minion/NewMinion_BP.bCanApplyBloodDrain` true _minionref)
          (`/Game/Blueprints/Minion/NewMinion_BP.ResetStatus` (`self.MinionRef`))))
      (`self.K2_DestroyActor`))
    (:`Landscape`
      (goto _label))))

(fn `BloodDrain`
  (`KismetSystemLibrary.PrintString` "Blood Drain"))

(fn `UserConstructionScript`
  (`parent.UserConstructionScript`))