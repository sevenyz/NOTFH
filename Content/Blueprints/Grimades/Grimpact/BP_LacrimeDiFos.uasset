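; BP_LacrimeDiFos is a fire grenade that explodes on impact, damaging bosses, the player and minions within its AOE by component tag.
; On a boss it either starts a looping Blaze burn, triggering delayed Toxicity if poisoned, or re-enables Blaze and resets status.
; The exploded actor hides its collider and stays alive to run the burn, destroying itself only when that ends, as its lifespan call is unconnected.
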(event `self.ReceiveBeginPlay`
  (`parent.ReceiveBeginPlay`))

(event `self.Collider.OnComponentHit`
  (params (HitComponent :type "PrimitiveComponent Object Reference") (OtherActor :type "Actor Object Reference") (OtherComp :type "PrimitiveComponent Object Reference") (NormalImpulse :type "Vector Structure") (Hit :type "HitResult Structure (by ref)"))
  (bind _bossref (`self.BossRef`))
  (bind _bossref_2 (`self.BossRef`))
  (bind _collider (`self.Collider`))
  (bind _bossref_3 (`self.BossRef`))
  (bind _bossref_4 (`self.BossRef`))
  (for _array_element (`PrimitiveComponent.GetOverlappingComponents` (`self.AOE`))
    (if (`ActorComponent.ComponentHasTag` _array_element "BossCollider")
      (set `Boss.bIsBombDamage` true _bossref)
      (`Boss.CalculateDamage` _bossref (`KismetMathLibrary.FTrunc` (`self.Damage`)))
      (if (`/Game/Blueprints/Boss/Boss_BP.bCanApplyBlaze` _bossref_2)
        (set `/Game/Blueprints/Boss/Boss_BP.bIsBlazeActive` true _bossref_4)
        (bind _returnvalue (`KismetSystemLibrary.K2_SetTimer` self "Blaze" 1.5 true))
        (set `self.TimerHandle` _returnvalue)
        (if (`/Game/Blueprints/Boss/Boss_BP.bIsPoisonActive` _bossref_4)
          (`KismetSystemLibrary.Delay` (`/Game/Blueprints/Boss/Boss_BP.ApplySynergyDelay` _bossref_3))
          (`/Game/Blueprints/Boss/Boss_BP.ToxicityTimer` _bossref_3))
        (else
          (set `/Game/Blueprints/Boss/Boss_BP.bCanApplyBlaze` true _bossref_2)
          (`/Game/Blueprints/Boss/Boss_BP.ResetStatus` _bossref_2)))
      (elif (`ActorComponent.ComponentHasTag` _array_element "PlayerCollider")
        (`FinalProjectAlphaCharacter.TakeDamage` (`self.PlayerRef`) (`KismetMathLibrary.FTrunc` (`self.Damage`)))
        (elif (`ActorComponent.ComponentHasTag` _array_element "MinionCollider")
          (bind _asnew_minion_bp (cast `/Game/Blueprints/Minion/NewMinion_BP` (`ActorComponent.GetOwner` _array_element)))
          (`NewMinion.CalculateDamage` _asnew_minion_bp (`KismetMathLibrary.FTrunc` (`self.Damage`)))))))
  (`GameplayStatics.SpawnEmitterAtLocation` "/Game/Particles/Explosion_Particle/Explosion.Explosion" (`self.K2_GetActorLocation`))
  (`PrimitiveComponent.SetCollisionEnabled` _collider "NoCollision")
  (`SceneComponent.SetVisibility` _collider false true))

(fn `Blaze`
  (bind _bossref (`self.BossRef`))
  (set `self.BlazeTimerCounter` (`self.BlazeTimerCounter`))
  (if (> (`self.BlazeTimerCounter`) 0)
    (`/Engine/EditorBlueprintResources/StandardMacros.DecrementInt` (`self.BlazeTimerCounter`)
      (:`  `
        (`KismetSystemLibrary.PrintString` "Blaze")
        (bind _output_get (set `Boss.CurrentHP` (- (`Boss.CurrentHP` _bossref) (`self.BlazeDamage`)) _bossref))
        (if (<= _output_get 0.0)
          (`Boss.Death` _bossref))))
    (else
      (`KismetSystemLibrary.PrintString` "Stop")
      (`KismetSystemLibrary.K2_ClearAndInvalidateTimerHandle` (`self.TimerHandle`))
      (set `/Game/Blueprints/Boss/Boss_BP.bIsBlazeActive` false (`self.BossRef`))
      (`self.K2_DestroyActor`))))

(fn `UserConstructionScript`
  (`parent.UserConstructionScript`))