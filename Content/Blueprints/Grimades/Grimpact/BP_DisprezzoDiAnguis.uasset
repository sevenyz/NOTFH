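; Grimade actor, Disprezzo Di Anguis, that spawns a SlowPuddle at the impact point when its Collider hits, then destroys itself.
; Its AOE overlaps set tagged boss, player and minion walk speeds to slowed on entry, if CheckOverlap is true, and back to chase or normal on exit.
; An unconnected chain that would enable CheckOverlap, slow current overlaps and destroy after Lifetime never runs.
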(event `self.ReceiveBeginPlay`
  (`parent.ReceiveBeginPlay`))

(event `self.Collider.OnComponentHit`
  (params (HitComponent :type "PrimitiveComponent Object Reference") (OtherActor :type "Actor Object Reference") (OtherComp :type "PrimitiveComponent Object Reference") (NormalImpulse :type "Vector Structure") (Hit :type "HitResult Structure (by ref)"))
  (`|SpawnActorFromClass` "/Game/Blueprints/Grimades/Grimpact/SlowPuddle.SlowPuddle_C" (`KismetMathLibrary.Conv_VectorToTransform` Hit_Location) "Undefined" "OverrideRootScale" null (0.0 0.0 0.0) null)
  (`self.K2_DestroyActor`))

(event `self.AOE.OnComponentBeginOverlap`
  (params (OverlappedComponent :type "PrimitiveComponent Object Reference") (OtherActor :type "Actor Object Reference") (OtherComp :type "PrimitiveComponent Object Reference") (OtherBodyIndex :type Integer) (bFromSweep :type Boolean) (SweepResult :type "HitResult Structure (by ref)"))
  (if (`self.CheckOverlap`)
    (`self.SetSlowedSpeed` OtherComp)))

(event `self.AOE.OnComponentEndOverlap`
  (params (OverlappedComponent :type "PrimitiveComponent Object Reference") (OtherActor :type "Actor Object Reference") (OtherComp :type "PrimitiveComponent Object Reference") (OtherBodyIndex :type Integer))
  (`self.SetNormalSpeed` OtherComp))

(fn `UserConstructionScript`
  (`parent.UserConstructionScript`))