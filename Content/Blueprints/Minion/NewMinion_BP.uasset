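; Wolf minion enemy with a health bar, hit, attack, trap and death animations, dropping magical essence when it dies.
; Combo hits restart a short timer, which then applies Bleeding, Blind or Poison by hit count, each with a health-bar icon.
; These statuses combine with Blaze, Frost and player Blood Drain into delayed synergies: Deep Wound, Toxicity, Heat Shock and Open Veins.
; Timers called by function name drive damage over time and most expiries.
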(event `self.ReceiveBeginPlay`
  (bind _asui_minion_hp (cast `/Game/Hud/UI_MinionHP` (`WidgetComponent.GetUserWidgetObject` (`self.HealthBarWidget`))))
  (set `/Game/Hud/UI_MinionHP.Minion` self _asui_minion_hp)
  (set `self.UIMinion2` _asui_minion_hp)
  (bind (_direction _newtrack_0) (`Timeline|Timeline_0`)
    (:`Update`
      (`SceneComponent.K2_SetRelativeLocation` (`self.Cone`) (`KismetMathLibrary.MakeVector` 0.0 0.0 _newtrack_0) false false))))

(event `AttackAnim`
  (bind _mesh (`self.Mesh`))
  (`|PlayMontage` _mesh "/Game/Characters/Minion/Animations/ANIM_Wolf_RunBite_RM_Montage.ANIM_Wolf_RunBite_RM_Montage"
    (:`OnCompleted`
      (`|PlayMontage` _mesh "/Game/Characters/Minion/Animations/ANIM_Wolf_stepback02_Montage.ANIM_Wolf_stepback02_Montage" 1.25
        (:`OnCompleted`
          (`SkeletalMeshComponent.SetAnimationMode` (`self.Mesh`) "AnimationBlueprint"))))))

(event `Trapped`
  (`SkeletalMeshComponent.PlayAnimation` (`self.Mesh`) "/Game/Characters/Minion/Animations/ANIM_Wolf_GetHitLeft.ANIM_Wolf_GetHitLeft" true)
  (`KismetSystemLibrary.Delay` (`self.StunTime`))
  (`SkeletalMeshComponent.SetAnimationMode` (`self.Mesh`) "AnimationBlueprint"))

(event `OnHit`
  (`SceneComponent.SetVisibility` (`self.HealthBarWidget`) true false)
  (`|PlayMontage` (`self.Mesh`) "/Game/Characters/Minion/Animations/ANIM_Wolf_GetHitRight_Montage.ANIM_Wolf_GetHitRight_Montage" 0.5
    (:`OnCompleted`
      (`SkeletalMeshComponent.SetAnimationMode` (`self.Mesh`) "AnimationBlueprint")
      (`BlackboardComponent.SetValueAsBool` (`AIBlueprintHelperLibrary.GetBlackboard` (`self.GetController`)) "IsHit" false)
      (`BlackboardComponent.SetValueAsBool` (`AIBlueprintHelperLibrary.GetBlackboard` (`self.GetController`)) "HasLineOfSight" true))))

(event `self.Death`
  (`/Engine/EditorBlueprintResources/StandardMacros.DoOnce` false
    (:`Completed`
      (`self.SetActorTickEnabled` false)
      (`self.DetachFromControllerPendingDestroy`)
      (`PrimitiveComponent.SetCollisionEnabled` (`self.Mesh`) "NoCollision")
      (`PrimitiveComponent.SetCollisionEnabled` (`self.CapsuleComponent`) "NoCollision")
      (bind _notifyname (`|PlayMontage` (`self.Mesh`) "/Game/Characters/Minion/Animations/ANIM_Wolf_Death_Montage.ANIM_Wolf_Death_Montage")
        (:`OnNotifyBegin`
          (if (== _notifyname "EndDeathAnimation")
            (`|SpawnActorFromClass` "/Game/Blueprints/BP_MagicalEssence.BP_MagicalEssence_C" (`KismetMathLibrary.Conv_VectorToTransform` (+ (`self.K2_GetActorLocation`) (0.0 0.0 50.0))) "Undefined" "OverrideRootScale" null null)
            (`SceneComponent.SetVisibility` (`self.Mesh`) false true)
            (`self.SetLifeSpan` 1.0)))))))

(event `ResetBleedingIcon`
  (`KismetSystemLibrary.Delay` 2.0)
  (`Widget.RemoveFromParent` (`self.BleedingIconWidget`)))

(event `ResetStatus`
  (`KismetSystemLibrary.Delay` (`self.ResetStatusDelay`))
  (set `self.bCanApplyBlaze` false)
  (set `self.bCanApplyBloodDrain` false)
  (set `self.bCanApplyFrost` false)
  (`KismetSystemLibrary.PrintString` "ResetStatus"))

(event `BlazeTimer`
  (set `self.BlazeTimerCounter` (`self.BlazeDuration`))
  (bind _returnvalue (`KismetSystemLibrary.K2_SetTimer` self "Blaze" 1.0 true))
  (set `self.BlazeTimerHandle` _returnvalue)
  (if (`self.bIsPoisonActive`)
    (`KismetSystemLibrary.Delay` (`self.ApplySynergyDelay`))
    (`self.ToxicityTimer`)))

(event `Frost`
  (params (LifeTime :type "Float (double-precision)"))
  (if (`self.bIsBlindActive`)
    (`KismetSystemLibrary.K2_SetTimer` self "HeatShock" (`self.ApplySynergyDelay`))
    (if (`self.bCanApplyFrost`)
      (set `self.bIsFrostActive` true)
      (`KismetSystemLibrary.PrintString` "Frost")
      (set `self.CustomTimeDilation` 0.5)
      (`KismetSystemLibrary.Delay` LifeTime)
      (set `self.CustomTimeDilation` 1.0)
      (set `self.bIsFrostActive` false)
      (else
        (set `self.bCanApplyFrost` true)
        (`self.ResetStatus`)))))

(fn `ApplyStatusEffect`
  (switch `int` (`self.ComboCount`)
    (:`Default`
      (`self.Poison` :!label _label))
    (:`1`
      _)
    (:`2`
      _)
    (:`3`
      (`self.Bleeding`))
    (:`4`
      (`self.Blind`))
    (:`5`
      (goto _label)))
  (set `self.ComboCount` 0)
  (`KismetSystemLibrary.PrintString` "end combo" true true (struct :`R` 1.0 :`B` 0.076571 :`A` 1.0)))

(fn `Blaze`
  (if (> (`self.BlazeTimerCounter`) 0)
    (`/Engine/EditorBlueprintResources/StandardMacros.DecrementInt` (`self.BlazeTimerCounter`)
      (:`  `
        (`KismetSystemLibrary.PrintString` "Blaze")
        (bind _output_get (set `self.CurrentHP` (- (`self.CurrentHP`) (`self.BlazeDamage`))))
        (if (<= _output_get 0.0)
          (`self.Death`))))
    (else
      (`KismetSystemLibrary.PrintString` "Stop")
      (`KismetSystemLibrary.K2_ClearAndInvalidateTimerHandle` (`self.BlazeTimerHandle`))
      (set `self.bIsBlazeActive` false))))

(fn `Bleeding`
  (locals (BleedingDamage :type "Float (double-precision)" :default 20.0))
  (bind _applysynergydelay (`self.ApplySynergyDelay`))
  (set `self.CurrentHP` (- (`self.CurrentHP`) (* (/ (`self.MaxHP`) 100.0) (`local.BleedingDamage`))))
  (bind _returnvalue (`|CreateWidget` "/Game/Hud/StatusIconsWidgets/BleedingIconWidget.BleedingIconWidget_C"))
  (bind _output_get (set `self.BleedingIconWidget` _returnvalue))
  (`HorizontalBox.AddChildToHorizontalBox` (`/Game/Hud/UI_MinionHP.Icons_HBox` (`self.UIMinion2`)) _output_get)
  (`self.ResetBleedingIcon`)
  (`GameplayStatics.SpawnEmitterAttached` "/Game/Particles/Blood/BloodSplat_PS.BloodSplat_PS" (`self.Mesh`) "pelvisSocket" (0.0 0.0 0.0) (struct) (0.5 0.5 0.5))
  (if (<= (`self.CurrentHP`) 0.0)
    (`self.Death`)
    (elif (`self.bIsPoisonActive`)
      (`KismetSystemLibrary.K2_SetTimer` self "DeepWound" _applysynergydelay true)
      (elif (`FinalProjectAlphaCharacter.bIsBloodDrainActive` (`self.PlayerRef`))
        (`KismetSystemLibrary.PrintString` "true")
        (`KismetSystemLibrary.K2_SetTimer` self "OpenVeins" _applysynergydelay)))))

(fn `Blind`
  (locals (BlindDuration :type "Float (double-precision)" :default 7.5))
  (set `self.bIsBlindActive` true)
  (if (`self.bIsFrostActive`)
    (`KismetSystemLibrary.K2_SetTimer` self "HeatShock" (`self.ApplySynergyDelay`)))
  (set `self.Damage` 0)
  (bind _returnvalue (`KismetSystemLibrary.K2_SetTimer` self "StopBlind" (`local.BlindDuration`)))
  (set `self.BlindTimerHandle` _returnvalue)
  (`KismetSystemLibrary.PrintString` "blind on")
  (bind _returnvalue_2 (`|CreateWidget` "/Game/Hud/StatusIconsWidgets/BlindIconWidget.BlindIconWidget_C"))
  (bind _output_get (set `self.BlindIconWidget` _returnvalue_2))
  (`HorizontalBox.AddChildToHorizontalBox` (`/Game/Hud/UI_MinionHP.Icons_HBox` (`self.UIMinion2`)) _output_get))

(fn `DecreaseHpOverTime`
  (if (>= (`self.PoisonTimerCounter`) (`self.PoisonDuration`))
    (`KismetSystemLibrary.K2_ClearAndInvalidateTimerHandle` (`self.PoisonTimerHandle`))
    (`KismetSystemLibrary.PrintString` "stop poison")
    (`Widget.RemoveFromParent` (`self.PoisonIconWidget`))
    (set `self.bIsPoisonActive` false)
    (else
      (`/Engine/EditorBlueprintResources/StandardMacros.IncrementFloat` (`self.PoisonTimerCounter`)
        (:`  `
          (bind _output_get (set `self.CurrentHP` (- (`self.CurrentHP`) (`self.PoisonDamage`))))
          (if (<= _output_get 0.0)
            (`self.Death`)))))))

(fn `DeepWound`
  (`KismetSystemLibrary.PrintString` "DeepWound")
  (bind _output_get (set `self.CurrentHP` (- (`self.CurrentHP`) (/ (- (`self.MaxHP`) (`self.CurrentHP`)) (`self.DeepWoundDamagePercentage`)))))
  (if (<= _output_get 0.0)
    (`self.Death`)))

(fn `HeatShock`
  (set `self.HeatShockDamage` (`self.HeatShockMultiplier`))
  (`KismetSystemLibrary.K2_SetTimer` self "StopHeatShock" (`self.HeatShockDuration`)))

(fn `IncrementComboCount`
  (bind _result (`/Engine/EditorBlueprintResources/StandardMacros.IncrementInt` (`self.ComboCount`))
    (:`  `
      (`KismetSystemLibrary.PrintString` (`KismetStringLibrary.Conv_IntToString` _result))
      (`KismetSystemLibrary.K2_ClearAndInvalidateTimerHandle` (`self.TimerHandle`))
      (bind _returnvalue (`KismetSystemLibrary.K2_SetTimer` self "ApplyStatusEffect" 2.0))
      (set `self.TimerHandle` _returnvalue))))

(fn `OpenVeins`
  (bind _playerref (`self.PlayerRef`))
  (bind _maxhp (`FinalProjectAlphaCharacter.MaxHP` _playerref))
  (bind _returnvalue (+ (* (/ _maxhp 100.0) (`self.OpenVeinsDamagePercentage`)) (`FinalProjectAlphaCharacter.CurrentHP` _playerref)))
  (set `self.CurrentHP` (- (`self.CurrentHP`) (* (/ (`self.MaxHP`) 100.0) (`self.OpenVeinsDamagePercentage`))))
  (bind _output_get (set `FinalProjectAlphaCharacter.CurrentHP` (select `bool` (<= _returnvalue _maxhp) :`false` _maxhp :`true` _returnvalue) _playerref))
  (`KismetSystemLibrary.PrintString` (`KismetStringLibrary.Conv_DoubleToString` _output_get))
  (if (<= (`self.CurrentHP`) 0.0)
    (`self.Death`)))

(fn `Poison`
  (set `self.bIsPoisonActive` true)
  (set `self.PoisonTimerCounter` 0.0)
  (`KismetSystemLibrary.K2_ClearAndInvalidateTimerHandle` (`self.PoisonTimerHandle`))
  (set `self.PoisonDamage` (* (`self.MaxHP`) (/ (`self.PoisonDamagePercentage`) 100.0)))
  (bind _returnvalue (`KismetSystemLibrary.K2_SetTimer` self "DecreaseHpOverTime" 0.5 true))
  (set `self.PoisonTimerHandle` _returnvalue)
  (bind _returnvalue_2 (`|CreateWidget` "/Game/Hud/StatusIconsWidgets/PoisonIconWidget.PoisonIconWidget_C"))
  (bind _output_get (set `self.PoisonIconWidget` _returnvalue_2))
  (`HorizontalBox.AddChildToHorizontalBox` (`/Game/Hud/UI_MinionHP.Icons_HBox` (`self.UIMinion2`)) _output_get)
  (if (`self.bIsBlazeActive`)
    (`KismetSystemLibrary.K2_SetTimer` self "ToxicityTimer" (`self.ApplySynergyDelay`))))

(fn `SetStatusIcon`
  (params (Index :type Integer))
  (returns (OutIndex :type Integer))
  (locals (LocalIndex :type Integer))
  (bind _uiminion (`self.UIMinion`))
  (bind _ws01 (`/Game/Hud/UI_MinionHP.WS01` _uiminion))
  (bind _ws02 (`/Game/Hud/UI_MinionHP.WS02` _uiminion))
  (bind _ws03 (`/Game/Hud/UI_MinionHP.WS03` _uiminion))
  (if (== (`WidgetSwitcher.GetActiveWidgetIndex` _ws01) 0)
    (`WidgetSwitcher.SetActiveWidgetIndex` _ws01 Index)
    (set `local.LocalIndex` 0)
    (return (`local.LocalIndex`))
    (elif (== (`WidgetSwitcher.GetActiveWidgetIndex` _ws02) 0)
      (`WidgetSwitcher.SetActiveWidgetIndex` _ws02 Index)
      (set `local.LocalIndex` 1)
      (return (`local.LocalIndex`))
      (elif (== (`WidgetSwitcher.GetActiveWidgetIndex` _ws03) 0)
        (`WidgetSwitcher.SetActiveWidgetIndex` _ws03 Index)
        (set `local.LocalIndex` 2)
        (return (`local.LocalIndex`))))))

(fn `StopBlind`
  (set `self.Damage` 10)
  (`KismetSystemLibrary.K2_ClearAndInvalidateTimerHandle` (`self.BlindTimerHandle`))
  (`KismetSystemLibrary.PrintString` "stop blind")
  (`Widget.RemoveFromParent` (`self.BlindIconWidget`))
  (set `self.bIsBlindActive` false))

(fn `StopHeatShock`
  (set `self.HeatShockDamage` 1.0))

(fn `Toxicity`
  (bind _toxicitytimercount (`self.ToxicityTimerCount`))
  (`KismetSystemLibrary.PrintString` "Toxicity" true true (struct :`R` 0.229663 :`G` 1.0 :`A` 1.0))
  (bind _output_get (set `self.ToxicityTimerCount` _toxicitytimercount))
  (if (> _output_get 0)
    (`/Engine/EditorBlueprintResources/StandardMacros.DecrementInt` _toxicitytimercount
      (:`  `
        (bind _output_get_2 (set `self.CurrentHP` (- (`self.CurrentHP`) (* (`self.MaxHP`) (/ (`self.ToxicityDOTPercentage`) 100.0)))))
        (if (<= _output_get_2 0.0)
          (`self.Death`))))
    (else
      (`KismetSystemLibrary.K2_ClearAndInvalidateTimerHandle` (`self.ToxicityTimerHandle`)))))

(fn `ToxicityTimer`
  (bind _output_get (set `self.CurrentHP` (- (`self.CurrentHP`) (`self.ToxicityInstantDamage`))))
  (if (<= _output_get 0.0)
    (`self.Death`)
    (else
      (bind _returnvalue (`KismetSystemLibrary.K2_SetTimer` self "Toxicity" 1.0 true))
      (set `self.ToxicityTimerHandle` _returnvalue))))

(fn `UpdateWalkSpeed`
  (params (NewSpeed :type "Float (double-precision)"))
  (set `CharacterMovementComponent.MaxWalkSpeed` NewSpeed (`self.CharacterMovement`)))

(fn `UserConstructionScript`)