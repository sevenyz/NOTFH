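; Wolf minion pawn Blueprint that plays animations for attacking, being trapped and dying, and exposes a walk speed setter for its movement component.
; Attack plays a jump bite, calls Attack and waits out the cooldown, while trapped loops a hit reaction for the stun time.
; Both then return the mesh to its Animation Blueprint, whereas death plays its animation and destroys the actor after a delay.
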(event `EventAttack`
  (`SkeletalMeshComponent.PlayAnimation` (`self.MyMesh`) "/Game/AnimalVarietyPack/Wolf/Animations/ANIM_Wolf_JumpBite.ANIM_Wolf_JumpBite" false)
  (`self.Attack`)
  (`KismetSystemLibrary.Delay` (`self.MinionCooldown`))
  (`SkeletalMeshComponent.SetAnimationMode` (`self.MyMesh`) "AnimationBlueprint" :!label _label))

(event `EventTrapped`
  (`SkeletalMeshComponent.PlayAnimation` (`self.MyMesh`) "/Game/AnimalVarietyPack/Wolf/Animations/ANIM_Wolf_GetHitLeft.ANIM_Wolf_GetHitLeft" true)
  (`KismetSystemLibrary.Delay` (`self.StunTime`))
  (goto _label))

(event `Death`
  (`SkeletalMeshComponent.PlayAnimation` (`self.MyMesh`) "/Game/AnimalVarietyPack/Wolf/Animations/ANIM_Wolf_Death.ANIM_Wolf_Death" false)
  (`KismetSystemLibrary.Delay` 5.0)
  (`self.K2_DestroyActor`))

(fn `UpdateWalkSpeed`
  (params (NewWalkSpeed :type "Float (double-precision)"))
  (set `FloatingPawnMovement.MaxSpeed` NewWalkSpeed (`self.PawnMovement`)))

(fn `UserConstructionScript`)