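; Lightsaber weapon that extends or retracts its blade and deals fixed damage to actors overlapping its capsule, excluding itself and its owner.
; TurnOn and TurnOff set target values for a shared timeline that lerps blade Z scale and point light intensity.
; Each Tick traces from blade base to tip, spawning spark and wall-burn emitters on hits, regardless of on/off state.
; SwitchLightsaberRibbon is unfinished, with its Activate and Deactivate calls disconnected.
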(event `self.ReceiveBeginPlay`
  (if (not (`self.IsTurnedOnByDefault`))
    (`self.TurnOff`)))

(event `self.ReceiveTick`
  (params (DeltaSeconds :type "Float (single-precision)"))
  (bind _blade (`self.Blade`))
  (bind _returnvalue (`KismetMathLibrary.Conv_DoubleToVector` (`KismetMathLibrary.RandomFloatInRange` 0.5 0.9)))
  (bind (_outhit _returnvalue_2) (`KismetSystemLibrary.LineTraceSingle` :`Start` (`SceneComponent.GetSocketLocation` _blade "Base") :`End` (`SceneComponent.GetSocketLocation` _blade "Tip") :`TraceChannel` "TraceTypeQuery1" :`DrawTime` 0.5))
  (if _returnvalue_2
    (bind (_bblockinghit _binitialoverlap _time _distance _location) (`GameplayStatics.BreakHitResult` _outhit))
    (`GameplayStatics.SpawnEmitterAtLocation` "/Game/Particles/LightsaberSparks.LightsaberSparks" _location (struct) _returnvalue)
    (`GameplayStatics.SpawnEmitterAtLocation` "/Game/Particles/LightsaberWallBurn.LightsaberWallBurn" _location (struct) _returnvalue)))

(event `TurnOn`
  (bind _pointlight (`self.PointLight`))
  (bind (_relativescale3d_x _relativescale3d_y _relativescale3d_z) (`KismetMathLibrary.BreakVector` (`SceneComponent.RelativeScale3D` (`self.Blade`))))
  (set `self.TargetBladeZScale` (`self.TurnedOnBladeZScale`))
  (set `self.TargetLightIntensity` (`self.TurnedOnLightIntensity`))
  (set `self.IsTurnedOn` true)
  ;[0 0 0] Extend/hide the blade
  (bind (_direction _alpha) (`Timeline|BladeTimeline` :!via `PlayFromStart` :!label _label)
    (:`Update`
      (`SceneComponent.SetRelativeScale3D` (`self.Blade`) (`KismetMathLibrary.MakeVector` _relativescale3d_x _relativescale3d_y (`KismetMathLibrary.Lerp` _relativescale3d_z (`self.TargetBladeZScale`) _alpha)))
      (`LightComponent.SetIntensity` _pointlight (`KismetMathLibrary.Lerp` (`LightComponentBase.Intensity` _pointlight) (`self.TargetLightIntensity`) _alpha)))))

(event `TurnOff`
  (set `self.TargetBladeZScale` 0.0)
  (set `self.TargetLightIntensity` 0.0)
  (set `self.IsTurnedOn` false)
  (goto _label :!via `PlayFromStart`))

(event `self.Capsule.OnComponentBeginOverlap`
  (params (OverlappedComponent :type "PrimitiveComponent Object Reference") (OtherActor :type "Actor Object Reference") (OtherComp :type "PrimitiveComponent Object Reference") (OtherBodyIndex :type Integer) (bFromSweep :type Boolean) (SweepResult :type "HitResult Structure (by ref)"))
  (if (and (!= OtherActor (`self.GetOwner`)) (!= OtherActor self))
    (`GameplayStatics.ApplyDamage` OtherActor 25.0 null self)))

(fn `SwitchLightsaberRibbon`
  (params (On :type Boolean))
  (if On
    _))

(fn `UserConstructionScript`)