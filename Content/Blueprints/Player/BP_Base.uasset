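; BP_Base is a player character Blueprint handling movement stances and basic sword combat.
; Input actions and matching custom events share macros for walk/run, crouch and weapon draw, while sprint sets speed directly.
; Drawing or sheathing plays a montage, then reattaches and moves the sword between hand and sheath.
; Light attack auto-draws before its montage; EnableAttack only prints Minions overlapping the attack collider.
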(event `InputAction|Toggle Walk/Run`
  (params (Key :type "Key Structure"))
  ;[1 1 1] Toggle Walk/Run
  (:`Pressed`
    (`self.Toggle Walk/Run M` (not (`self.bIsRunning`)))))

(event `/Game/Blueprints/Player/BPInterface_CharacterActions.RunOn`
  (params (Enabled :type Boolean))
  ;[1 1 1] Toggle Walk/Run
  (`self.Toggle Walk/Run M` Enabled))

(event `InputAction|Sprint`
  (params (Key :type "Key Structure"))
  ;[1 1 1] Sprinting
  (:`Pressed`
    (set `self.bIsSprinting` true :!label _label)
    (set `CharacterMovementComponent.MaxWalkSpeed` 900.0 (`self.CharacterMovement`))
    (`/Game/Blueprints/Player/BPInterface_CharacterActions.CrouchOn` false))
  (:`Released`
    (set `self.bIsSprinting` false :!label _label_2)
    (set `CharacterMovementComponent.MaxWalkSpeed` 600.0 (`self.CharacterMovement`))
    (set `self.bIsRunning` true)))

(event `/Game/Blueprints/Player/BPInterface_CharacterActions.SprintOn`
  (params (Enabled :type Boolean))
  ;[1 1 1] Sprinting
  (if Enabled
    (goto _label)
    (else
      (goto _label_2))))

(event `InputAction|Crouch`
  (params (Key :type "Key Structure"))
  ;[1 1 1] Crouch
  (:`Pressed`
    (`self.Crouch M` (not (`self.bIsCrouching`)))))

(event `/Game/Blueprints/Player/BPInterface_CharacterActions.CrouchOn`
  (params (Enabled :type Boolean))
  ;[1 1 1] Crouch
  (`self.Crouch M` Enabled))

(event `InputAction|Draw Weapon`
  (params (Key :type "Key Structure"))
  ;[1 1 1] Draw Weapon
  (:`Pressed`
    (`self.Draw Weapon M` (not (`self.bIsWeaponDrawn`)))))

(event `/Game/Blueprints/Player/BPInterface_CharacterActions.WeaponOn`
  (params (Drawn :type Boolean))
  ;[1 1 1] Draw Weapon
  (`self.Draw Weapon M` Drawn))

(event `InputAction|Light Attack`
  (params (Key :type "Key Structure"))
  (:`Pressed`
    (if (not (`self.bIsWeaponDrawn`))
      (`self.Draw Weapon M` true
        (:`Completed`
          _)))
    (`|PlayMontage` (`self.Mesh`) "/Game/Animations/Combat/Light_Attack_1_Montage.Light_Attack_1_Montage" 1.5)))

(event `EnableAttack`
  (for _array_element (`PrimitiveComponent.GetOverlappingActors` (`self.AttackCollider`) "/Script/FinalProjectAlpha.Minion")
    (`KismetSystemLibrary.PrintString` (`KismetSystemLibrary.GetDisplayName` _array_element))))

(fn `UserConstructionScript`)