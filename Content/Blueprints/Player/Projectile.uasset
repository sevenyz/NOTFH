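; Player projectile Blueprint that hands its initial speed to BP_Player on BeginPlay and holds disconnected trap-placement logic.
; The Sphere1 hit event is empty, so the spawn chain never runs.
; That chain would spawn the selected damage, stun or slow trap where it hits Landscape-tagged actors, refund the trap counter if spawning fails, then destroy the projectile.
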(event `self.ReceiveBeginPlay`
  (bind _asbp_player (cast `/Game/Blueprints/Player/BP_Player` (`GameplayStatics.GetPlayerCharacter` 0)))
  (bind _output_get (set `self.PlayerRef` _asbp_player))
  (set `/Game/Blueprints/Player/BP_Player.ProjectileSpeed` (`ProjectileMovementComponent.InitialSpeed` (`self.ProjectileMovement`)) _output_get))

(event `self.Sphere1.OnComponentHit`
  (params (HitComponent :type "PrimitiveComponent Object Reference") (OtherActor :type "Actor Object Reference") (OtherComp :type "PrimitiveComponent Object Reference") (NormalImpulse :type "Vector Structure") (Hit :type "HitResult Structure (by ref)")))

(fn `UserConstructionScript`)