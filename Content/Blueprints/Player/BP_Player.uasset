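; Player character Blueprint for melee combat against minions and a boss, with target lock-on, walk/run and crouch.
; A sphere collects tagged enemies; lock-on picks the nearest visible one, switching follows array order, and timelines turn the camera boom toward the target.
; Montages drive attacks, hit reactions and invulnerable dodge/stepback, using state flags to gate input.
; EnableAttack damages collider overlaps; weapon-draw, roll and strafe-style facing code is unwired.
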(event `self.ReceiveBeginPlay`
  (bind _outactors (`GameplayStatics.GetAllActorsOfClass` "/Game/Blueprints/Boss/Boss_BP.Boss_BP_C"))
  (set `self.Boss` (`|GetArrayItem` _outactors)))

(event `self.Sphere.OnComponentBeginOverlap`
  (params (OverlappedComponent :type "PrimitiveComponent Object Reference") (OtherActor :type "Actor Object Reference") (OtherComp :type "PrimitiveComponent Object Reference") (OtherBodyIndex :type Integer) (bFromSweep :type Boolean) (SweepResult :type "HitResult Structure (by ref)"))
  ;[0 0 0] Target Lock
  (if (`self.ActorHasTag` OtherActor "Minion")
    (bind _asnew_minion_bp (cast `/Game/Blueprints/Minion/NewMinion_BP` OtherActor))
    (`KismetArrayLibrary.Array_Add` (`self.EnemyArray`) _asnew_minion_bp)
    (elif (`self.ActorHasTag` OtherActor "Boss")
      (`KismetArrayLibrary.Array_Add` (`self.EnemyArray`) (`self.Boss`)))))

(event `self.Sphere.OnComponentEndOverlap`
  (params (OverlappedComponent :type "PrimitiveComponent Object Reference") (OtherActor :type "Actor Object Reference") (OtherComp :type "PrimitiveComponent Object Reference") (OtherBodyIndex :type Integer))
  (bind _boss (`self.Boss`))
  ;[0 0 0] Target Lock
  (if (`self.ActorHasTag` OtherActor "Minion")
    (bind _asnew_minion_bp (cast `/Game/Blueprints/Minion/NewMinion_BP` OtherActor))
    (if (!= (`KismetArrayLibrary.Array_Find` (`self.EnemyArray`) _asnew_minion_bp) -1)
      (`KismetArrayLibrary.Array_RemoveItem` (`self.EnemyArray`) _asnew_minion_bp)
      (if (== _asnew_minion_bp (`self.LockedOnEnemy`))
        (`self.ResetCamera`)))
    (elif (`self.ActorHasTag` OtherActor "Boss")
      (if (!= (`KismetArrayLibrary.Array_Find` (`self.EnemyArray`) (`self.Boss`)) -1)
        (`KismetArrayLibrary.Array_RemoveItem` (`self.EnemyArray`) _boss)
        (if (== _boss (`self.LockedOnEnemy`))
          (`self.ResetCamera`))))))

(event `InputAction|LockOn`
  (params (Key :type "Key Structure"))
  ;[0 0 0] Target Lock
  (:`Pressed`
    (if (`self.bIsLocked`)
      (if (>= (`KismetArrayLibrary.Array_Length` (`self.EnemyArray`)) 1)
        (switch `int` (`KismetArrayLibrary.Array_Length` (`self.EnemyArray`))
          (:`Default`
            _)
          (:`0`
            _)
          (:`1`
            _))
        (`self.ResetCamera`))
      (elif (>= (`KismetArrayLibrary.Array_Length` (`self.EnemyArray`)) 1)
        (`self.SelectEnemy`)
        (`/Engine/EditorBlueprintResources/StandardMacros.IsValid` (`self.LockedOnEnemy`)
          (:`Is Valid`
            (set `self.bIsLocked` true)
            (`self.RotateCamera`)
            (set `SpringArmComponent.bUsePawnControlRotation` false (`self.CameraBoom`))
            (set `SpringArmComponent.TargetArmLength` 450.0 (`self.CameraBoom`))
            (`CameraComponent.SetFieldOfView` (`self.FollowCamera`) 90.0)))))))

(event `InputAction|SwitchTarget`
  (params (Key :type "Key Structure"))
  ;[0 0 0] Target Lock
  (:`Pressed`
    (if (`self.bIsLocked`)
      (if (> (`KismetArrayLibrary.Array_Length` (`self.EnemyArray`)) 1)
        (`self.SelectEnemy`)
        (`self.ChangeEnemy`)))))

(event `ResetCamera`
  (bind _lockedonenemy (`self.LockedOnEnemy`))
  (bind _cameraboom (`self.CameraBoom`))
  ;[0 0 0] Target Lock
  (`/Engine/EditorBlueprintResources/StandardMacros.IsValid` _lockedonenemy
    (:`Is Valid`
      (if (`self.ActorHasTag` _lockedonenemy "Minion")
        (bind _asnew_minion_bp (cast `/Game/Blueprints/Minion/NewMinion_BP` _lockedonenemy))
        (`SceneComponent.SetVisibility` (`/Game/Blueprints/Minion/NewMinion_BP.Cone` _asnew_minion_bp) false false)
        (set `self.LockedOnEnemy` null :!label _label)
        (set `self.bIsLocked` false)
        (`Controller.SetControlRotation` (`GameplayStatics.GetPlayerController` 0) (`SceneComponent.K2_GetComponentRotation` (`self.CameraBoom`)))
        (set `SpringArmComponent.bUsePawnControlRotation` true _cameraboom)
        (set `SpringArmComponent.TargetArmLength` 500.0 _cameraboom)
        (`CameraComponent.SetFieldOfView` (`self.FollowCamera`) 80.0)
        (elif (`self.ActorHasTag` _lockedonenemy "Boss")
          (`SceneComponent.SetVisibility` (`/Game/Blueprints/Boss/Boss_BP.Cone` (`self.Boss`)) false false)
          (goto _label))))))

(event `RotateCamera`
  ;[0 0 0] Target Lock
  (`Timeline|Timeline_0` :!label _label_2
    (:`Update`
      (`/Engine/EditorBlueprintResources/StandardMacros.IsValid` (`self.LockedOnEnemy`)
        (:`Is Valid`
          (`self.RotateToTarget` :!label _label_3))))))

(event `ChangeEnemy`
  ;[0 0 0] Target Lock
  (`|ExecutionSequence`
    (:`then_0`
      (goto _label_2 :!via `Stop`))
    (:`then_1`
      (`Timeline|Timeline_1`
        (:`Update`
          (`/Engine/EditorBlueprintResources/StandardMacros.IsValid` (`self.LockedOnEnemy`)
            (:`Is Valid`
              (goto _label_3))))
        (:`Finished`
          (goto _label_2))))))

(event `InputAction|Toggle Walk/Run`
  (params (Key :type "Key Structure"))
  ;[0 0 0] Toggle Walk/Run
  (:`Pressed`
    (`self.Toggle Walk/Run M` (not (`self.bIsRunning`)))))

(event `/Game/Blueprints/Player/BPInterface_CharacterActions.RunOn`
  (params (Enabled :type Boolean))
  ;[0 0 0] Toggle Walk/Run
  (`self.Toggle Walk/Run M` Enabled))

(event `InputAction|Sprint`
  (params (Key :type "Key Structure"))
  ;[0 0 0] Sprinting
)

(event `/Game/Blueprints/Player/BPInterface_CharacterActions.SprintOn`
  (params (Enabled :type Boolean))
  ;[0 0 0] Sprinting
  (if Enabled
    (set `self.bIsSprinting` true)
    (`/Game/Blueprints/Player/BPInterface_CharacterActions.CrouchOn` false)
    (else
      (set `self.bIsSprinting` false)
      (set `self.bIsRunning` true))))

(event `InputAction|Crouch`
  (params (Key :type "Key Structure"))
  ;[0 0 0] Crouch
  (:`Pressed`
    (`self.Crouch M` (not (`self.bIsCrouching`)))))

(event `/Game/Blueprints/Player/BPInterface_CharacterActions.CrouchOn`
  (params (Enabled :type Boolean))
  ;[0 0 0] Crouch
  (`self.Crouch M` Enabled))

(event `InputAction|Draw Weapon`
  (params (Key :type "Key Structure"))
  ;[0 0 0] Draw Weapon
)

(event `/Game/Blueprints/Player/BPInterface_CharacterActions.WeaponOn`
  (params (Drawn :type Boolean))
  ;[0 0 0] Draw Weapon
)

(event `InputAction|Light Attack`
  (params (Key :type "Key Structure"))
  ;[0 0 0] Attack
  (:`Pressed`
    (if (and (and (not (`self.bIsAttacking`)) (not (`self.bIsCraftingPanelOpen`))) (not (`self.bIsHit`)))
      (if (not (`self.bIsDodging`))
        (`self.SetMovement` 0.0)
        (bind _notifyname (`|PlayMontage` (`self.Mesh`) "/Game/Character/RedHood/Animations/Attacco_Montage.Attacco_Montage" 1.5)
          (:`then`
            (set `self.bIsAttacking` true)
            (bind _result (`/Engine/EditorBlueprintResources/StandardMacros.IncrementInt` (`self.ComboCount`))
              (:`  `
                (`KismetSystemLibrary.PrintString` (`KismetStringLibrary.Conv_IntToString` _result)))))
          (:`OnCompleted`
            (set `self.ComboCount` 0))
          (:`OnNotifyEnd`
            (if (== _notifyname "Attack")
              (`self.CanAttackAgain`))))))))

(event `EnableAttack`
  ;[0 0 0] Enabling the attack: Method 1
  (for _array_element (`PrimitiveComponent.GetOverlappingActors` (`self.AttackCollider`) "/Script/Engine.Character")
    (if (`self.ActorHasTag` _array_element "Minion")
      (bind _asnew_minion_bp (cast `/Game/Blueprints/Minion/NewMinion_BP` _array_element))
      (`NewMinion.CalculateDamage` _asnew_minion_bp (`self.Damage`))
      (elif (`self.ActorHasTag` _array_element "Boss")
        (bind _asboss_bp (cast `/Game/Blueprints/Boss/Boss_BP` _array_element))
        (if (not (`/Game/Blueprints/Boss/Boss_BP.bIsHit` _asboss_bp))
          (`Boss.CalculateDamage` _asboss_bp (`self.DamageToBoss`) (`self.DamageIfBossStunned`)))))))

(event `self.TakeDamage`
  (params (DamageToTake :type Integer))
  ;[0 0 0] Take Damage
  (if (`self.bCanTakeDamage`)
    (if (> (`self.CurrentHP`) 0)
      (set `self.bIsHit` true)
      (set `self.CurrentHP` (- (`self.CurrentHP`) DamageToTake))
      (`|PlayMontage` (`self.Mesh`) "/Game/Character/RedHood/Animations/GotHit_Montage.GotHit_Montage" 0.6
        (:`then`
          (`KismetSystemLibrary.PrintString` "Take damage")
          (`self.SetMovement` 0.0)
          (set `self.ComboCount` 0))
        (:`OnCompleted`
          (set `self.bIsAttacking` false :!label _label)
          (set `self.bIsHit` false)
          (if (`self.bIsRunning`)
            (`self.SetMovement` 600.0 (struct :`Yaw` 540.0))
            (else
              (`self.SetMovement` 300.0 (struct :`Yaw` 540.0))))))
      (else
        (`KismetSystemLibrary.PrintString` "player dead")))
    (else
      (goto _label))))

(event `Key|SpaceBar`
  (params (Key :type "Key Structure"))
  ;[0 0 0] Roll test
)

(event `InputAction|Dodge/StepBack`
  (params (Key :type "Key Structure"))
  (bind _mesh (`self.Mesh`))
  ;[0 0 0] Dodge/Stepback
  (:`Pressed`
    (if (and (and (not (`self.bIsAttacking`)) (not (`self.bIsHit`))) (not (`self.bIsDodging`)))
      (set `self.bCanTakeDamage` false)
      (set `self.bIsDodging` true)
      (if (!= (`self.GetVelocity`) (0.0 0.0 0.0))
        (`|PlayMontage` _mesh "/Game/Character/RedHood/Animations/RootMotion/Dodge_Montage.Dodge_Montage" 1.3
          (:`OnCompleted`
            _))
        (else
          (`|PlayMontage` _mesh "/Game/Character/RedHood/Animations/RootMotion/Stepback_Montage.Stepback_Montage"
            (:`OnCompleted`
              _))))
      (set `self.bCanTakeDamage` true)
      (set `self.bIsDodging` false))))

(fn `RotateToTarget`
  (bind (_returnvalue_roll _returnvalue_pitch _returnvalue_yaw) (`KismetMathLibrary.BreakRotator` (`KismetMathLibrary.FindLookAtRotation` (`KismetMathLibrary.MakeVector` (.x (`SceneComponent.K2_GetComponentLocation` (`self.CameraBoom`))) (.y (`SceneComponent.K2_GetComponentLocation` (`self.CameraBoom`)))) (`KismetMathLibrary.MakeVector` (.x (`self.K2_GetActorLocation` (`self.LockedOnEnemy`))) (.y (`self.K2_GetActorLocation` (`self.LockedOnEnemy`)))))))
  ;[0 0 0] Free Movement
  (`SceneComponent.K2_SetWorldRotation` (`self.CameraBoom`) (`KismetMathLibrary.MakeRotator` _returnvalue_roll -10.0 _returnvalue_yaw) false false))

(fn `SelectEnemy`
  (locals (LastEnemy :type "Character Object Reference") (EnemiesDinstaces :type "Map of Float (double-precision) to Character Object Reference"))
  (bind _lastenemy (`local.LastEnemy`))
  (bind _output (`|GetArrayItem` (`self.EnemyArray`)))
  (bind _output_2 (`|GetArrayItem` (`self.EnemyArray`) (+ (`KismetArrayLibrary.Array_Find` (`self.EnemyArray`) (`self.LockedOnEnemy`)) 1)))
  (set `local.LastEnemy` (`self.LockedOnEnemy`))
  (for _array_element (`self.EnemyArray`)
    (`/Engine/EditorBlueprintResources/StandardMacros.IsValid` _array_element
      (:`Is Valid`
        (bind (_outhit _returnvalue) (`KismetSystemLibrary.LineTraceSingle` (`self.K2_GetActorLocation`) (`self.K2_GetActorLocation` _array_element) "TraceTypeQuery1"))
        (if (not _returnvalue)
          (`BlueprintMapLibrary.Map_Add` (`local.EnemiesDinstaces`) (`self.GetDistanceTo` _array_element self) _array_element)))))
  (if (`self.bIsLocked`)
    (bind _values (`BlueprintMapLibrary.Map_Values` (`local.EnemiesDinstaces`)))
    (`/Engine/EditorBlueprintResources/StandardMacros.IsValid` _output_2
      (:`Is Valid`
        (if (`KismetArrayLibrary.Array_Contains` _values _output_2)
          (`self.SetEnemy` _output_2)
          (if (`self.ActorHasTag` _lastenemy "Minion") :!label _label
            (bind _asnew_minion_bp (cast `/Game/Blueprints/Minion/NewMinion_BP` _lastenemy))
            (`SceneComponent.SetVisibility` (`/Game/Blueprints/Minion/NewMinion_BP.Cone` _asnew_minion_bp) false false)
            (elif (`self.ActorHasTag` _lastenemy "Boss")
              (`SceneComponent.SetVisibility` (`/Game/Blueprints/Boss/Boss_BP.Cone` (`self.Boss`)) false false)))
          (else
            (`self.ResetCamera` :!label _label_2))))
      (:`Is Not Valid`
        (if (`KismetArrayLibrary.Array_Contains` _values _output)
          (`self.SetEnemy` _output)
          (goto _label)
          (else
            (goto _label_2)))))
    (else
      (bind _keys (`BlueprintMapLibrary.Map_Keys` (`local.EnemiesDinstaces`)))
      (bind _value (`BlueprintMapLibrary.Map_Find` (`local.EnemiesDinstaces`) (`.MinValue` (`KismetMathLibrary.MinOfFloatArray` _keys))))
      (`/Engine/EditorBlueprintResources/StandardMacros.IsValid` _value
        (:`Is Valid`
          (`self.SetEnemy` _value))))))

(fn `SetEnemy`
  (params (EnemyToLock :type "Character Object Reference"))
  (bind _output_get (set `self.LockedOnEnemy` EnemyToLock))
  (if (`self.ActorHasTag` _output_get "Minion")
    (bind _asnew_minion_bp (cast `/Game/Blueprints/Minion/NewMinion_BP` _output_get))
    (`SceneComponent.SetVisibility` (`/Game/Blueprints/Minion/NewMinion_BP.Cone` _asnew_minion_bp) true false)
    (elif (`self.ActorHasTag` _output_get "Boss")
      (`SceneComponent.SetVisibility` (`/Game/Blueprints/Boss/Boss_BP.Cone` (`self.Boss`)) true false))))

(fn `SetMovement`
  (params (MaxWalkSpeed :type "Float (double-precision)") (RotationRate :type "Rotator Structure"))
  (bind _charactermovement (`self.CharacterMovement`))
  (set `CharacterMovementComponent.MaxWalkSpeed` MaxWalkSpeed _charactermovement)
  (set `CharacterMovementComponent.RotationRate` RotationRate _charactermovement)
  (return))

(fn `UserConstructionScript`)