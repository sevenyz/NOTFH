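; Minion character Blueprint for an AI-controlled enemy or unit that uses wolf animations and shows a health bar widget bound to itself.
; Events play attack, trap-stun and hit reactions, then restore Animation Blueprint mode, with the hit reaction also clearing the Blackboard IsHit flag.
; Death runs once, detaching the controller and disabling collision during the montage, then destroying the actor.
; A helper function sets walk speed.
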(event `self.ReceiveBeginPlay`
  (bind _asui_minion_hp (cast `/Game/Hud/UI_MinionHP` (`WidgetComponent.GetUserWidgetObject` (`self.HealthBarWidget`))))
  (set `/Game/Hud/UI_MinionHP.Minion` self _asui_minion_hp))

(event `AttackAnim`
  (`|PlayMontage` (`self.Mesh`) "/Game/AnimalVarietyPack/Wolf/Animations/ANIM_Wolf_JumpBite_Montage2.ANIM_Wolf_JumpBite_Montage2"
    (:`OnCompleted`
      (`SkeletalMeshComponent.SetAnimationMode` (`self.Mesh`) "AnimationBlueprint"))))

(event `Trapped`
  (`SkeletalMeshComponent.PlayAnimation` (`self.Mesh`) "/Game/AnimalVarietyPack/Wolf/Animations/ANIM_Wolf_GetHitLeft.ANIM_Wolf_GetHitLeft" true)
  (`KismetSystemLibrary.Delay` (`self.StunTime`))
  (`SkeletalMeshComponent.SetAnimationMode` (`self.Mesh`) "AnimationBlueprint"))

(event `OnHit`
  (`|PlayMontage` (`self.Mesh`) "/Game/AnimalVarietyPack/Wolf/Animations/ANIM_Wolf_GetHitRight_Montage.ANIM_Wolf_GetHitRight_Montage" 0.5
    (:`OnCompleted`
      (`SkeletalMeshComponent.SetAnimationMode` (`self.Mesh`) "AnimationBlueprint")
      (`BlackboardComponent.SetValueAsBool` (`AIBlueprintHelperLibrary.GetBlackboard` (`self.GetController`)) "IsHit" false))))

(event `self.Death`
  (`/Engine/EditorBlueprintResources/StandardMacros.DoOnce` false
    (:`Completed`
      (`|PlayMontage` (`self.Mesh`) "/Game/AnimalVarietyPack/Wolf/Animations/ANIM_Wolf_Death_Montage.ANIM_Wolf_Death_Montage"
        (:`then`
          (`self.DetachFromControllerPendingDestroy`)
          (`PrimitiveComponent.SetCollisionEnabled` (`self.Mesh`) "NoCollision")
          (`PrimitiveComponent.SetCollisionEnabled` (`self.CapsuleComponent`) "NoCollision"))
        (:`OnCompleted`
          (`self.K2_DestroyActor`))))))

(fn `UpdateWalkSpeed`
  (params (NewSpeed :type "Float (double-precision)"))
  (set `CharacterMovementComponent.MaxWalkSpeed` NewSpeed (`self.CharacterMovement`)))

(fn `UserConstructionScript`)